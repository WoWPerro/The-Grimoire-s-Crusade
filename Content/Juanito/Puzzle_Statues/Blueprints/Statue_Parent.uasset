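; Base statue actor for a hit-the-statues puzzle linked to a door (Puerta).
; Damage of the player damage type passes a DoOnce gate, sets GotHit and reports the statue's type to the door.
; OnfailEvent clears GotHit and resets the gate so the statue can be hit again.
; GotHit's RepNotify calls MaterialNotify, which only prints a debug string here.
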(event Custom|OnfailEvent
  (Development|PrintString "hahaha")
  (Variables|Default|SetGotHit false)
  (Utilities|FlowControl|DoOnce false) ; enters at Reset
)

(event Custom|MaterialNotify
  (Development|PrintString "unu"))

(event Game|Damage|EventAnyDamage
  (params (Damage :type Float%20%28single-precision%29) (DamageType :type Damage%20Type%20Object%20Reference) (InstigatedBy :type Controller%20Object%20Reference) (DamageCauser :type Actor%20Object%20Reference))
  (Utilities|Casting|CastToPlayerDMG_Type DamageType)
  (Utilities|FlowControl|DoOnce false
    (:Completed
      (Variables|Default|SetGotHit true)
      (Default|StatueHit (Variables|Default|GetPuerta) (Variables|Default|GetStatueType)))))

(fn ConstructionScript)

(fn OnRepGotHit
  (CallFunction|MaterialNotify))