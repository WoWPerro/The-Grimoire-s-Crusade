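; Fire variant of a puzzle statue that gives color feedback by swapping the material on its Statue component.
; It extends the parent's fail event with Fallando, which shows red for two seconds, restores the default fire material and prints a debug string.
; MaterialNotify switches the statue to green with no timed reset.
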(event Custom|Fallando
  (Rendering|Material|SetMaterial (Variables|Default|GetStatue) 0 "/Game/Juanito/Puzzle_Statues/Materiales/Mats/Statue_FireMatMaster_Red.Statue_FireMatMaster_Red")
  (Utilities|FlowControl|Delay 2.0)
  (Rendering|Material|SetMaterial (Variables|Default|GetStatue) 0 "/Game/Juanito/Puzzle_Statues/Materiales/Mats/Statue_FireMatMaster.Statue_FireMatMaster")
  (Development|PrintString "zamaHello"))

(event EventOnfailEvent
  (|CallParentFunction)
  (CallFunction|Fallando))

(event EventMaterialNotify
  (Rendering|Material|SetMaterial (Variables|Default|GetStatue) 0 "/Game/Juanito/Puzzle_Statues/Materiales/Mats/Statue_FireMatMaster_Green.Statue_FireMatMaster_Green"))

(fn ConstructionScript
  (|CallParentFunction))